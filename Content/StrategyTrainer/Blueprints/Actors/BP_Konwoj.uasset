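; BP_Konwoj is the blue convoy actor in the strategy trainer, registered as a Learning Agents agent, with a unit lineup built from an enum array.
; A looping timer resolves one queued engagement at a time, rolling kill chances to damage the front convoy unit and the queued red unit.
; Hits and deaths spawn short-lived effect actors and log to statistics widgets; losing every unit resets the convoy through BP_RoadSpline.
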(event `OnDeath`
  (bind (_returnvalue_location _returnvalue_rotation) (`KismetMathLibrary.BreakTransform` (`SceneComponent.K2_GetComponentToWorld` (`self.Scene`))))
  (bind _returnvalue (`|SpawnActorFromClass` "/Game/StrategyTrainer/Blueprints/Actors/BP_AnimationMesh.BP_AnimationMesh_C" (`KismetMathLibrary.MakeTransform` _returnvalue_location _returnvalue_rotation) "AlwaysSpawn" "MultiplyWithRoot" null null))
  (`SkeletalMeshComponent.SetAnimation` (`/Game/StrategyTrainer/Blueprints/Actors/BP_AnimationMesh.SkeletalMesh` _returnvalue) "/Game/StrategyTrainer/Animations/Convoy_BoomPow_effect4_Anim_Boom.Convoy_BoomPow_effect4_Anim_Boom")
  (`self.SetLifeSpan` _returnvalue 0.5))

(event `Hit`
  (bind (_returnvalue_location _returnvalue_rotation) (`KismetMathLibrary.BreakTransform` (`SceneComponent.K2_GetComponentToWorld` (`self.Scene`))))
  (bind _returnvalue (`|SpawnActorFromClass` "/Game/StrategyTrainer/Blueprints/Actors/BP_AnimationMesh.BP_AnimationMesh_C" (`KismetMathLibrary.MakeTransform` _returnvalue_location _returnvalue_rotation) "AlwaysSpawn" "MultiplyWithRoot" null null))
  (`self.SetLifeSpan` _returnvalue 0.4))

(event `self.ReceiveBeginPlay`
  (bind _returnvalue (`GameplayStatics.GetActorOfClass` "/Game/StrategyTrainer/Blueprints/Actors/BP_RoadSpline.BP_RoadSpline_C"))
  (set `self.RoadSpline` _returnvalue)
  (bind _returnvalue_2 (`GameplayStatics.GetActorOfClass` "/Game/StrategyTrainer/Blueprints/Actors/BP_KonwojManager.BP_KonwojManager_C"))
  (`LearningAgentsManager.AddAgent` (`/Game/StrategyTrainer/Blueprints/Actors/BP_KonwojManager.LearningAgentsManager` _returnvalue_2) self)
  (bind _returnvalue_3 (`KismetSystemLibrary.K2_SetTimerDelegate` (delegate `Battle`) 0.7 true true))
  (set `self.BattleTimerHandle` _returnvalue_3)
  (add `/Game/StrategyTrainer/Blueprints/GameModes/GM_StrategyTrainer.OnRoundEnd` (cast `/Game/StrategyTrainer/Blueprints/GameModes/GM_StrategyTrainer` (`GameplayStatics.GetGameMode`) :!pure true) (delegate `OnRoundEnd_Event`)))

(event `OnRoundEnd_Event`
  (`KismetArrayLibrary.Array_Clear` (`self.BattleQueue`)))

(event `AddBattleQueue`
  (params (NewItem :type "/Game/StrategyTrainer/Blueprints/Types/S_BattleQueueEntry Structure (by ref)"))
  (`KismetArrayLibrary.Array_Add` (`self.BattleQueue`) NewItem))

(event `Battle`
  (bind _battlequeue (`self.BattleQueue`))
  (bind _settings_konwojsettingentries (break `/Game/StrategyTrainer/Blueprints/Types/S_KonwojSettings` (`self.Settings`)))
  (bind _battlequeue_2 (`self.BattleQueue`))
  (bind _settings_konwojsettingentries_2 (break `/Game/StrategyTrainer/Blueprints/Types/S_KonwojSettings` (`self.Settings`)))
  (bind _settings_konwojsettingentries_3 (break `/Game/StrategyTrainer/Blueprints/Types/S_KonwojSettings` (`self.Settings`)))
  (bind _settings_konwojsettingentries_4 (break `/Game/StrategyTrainer/Blueprints/Types/S_KonwojSettings` (`self.Settings`)))
  (bind _settings_konwojsettingentries_5 (break `/Game/StrategyTrainer/Blueprints/Types/S_KonwojSettings` (`self.Settings`)))
  (bind _settings_konwojsettingentries_6 (break `/Game/StrategyTrainer/Blueprints/Types/S_KonwojSettings` (`self.Settings`)))
  (bind (_output_unitclass _output_hp) (break `/Game/StrategyTrainer/Blueprints/Types/S_KonwojSettingEntry` (`|GetArrayItem` _settings_konwojsettingentries_4)))
  (bind (_output_blueunit _output_redunit) (break `/Game/StrategyTrainer/Blueprints/Types/S_BattleQueueEntry` (`|GetArrayItem` _battlequeue)))
  (bind (_output_blueunit_2 _output_redunit_2) (break `/Game/StrategyTrainer/Blueprints/Types/S_BattleQueueEntry` (`|GetArrayItem` (`self.BattleQueue`))))
  (bind _output_unitclass_2 (break `/Game/StrategyTrainer/Blueprints/Types/S_KonwojSettingEntry` (`|GetArrayItem` _settings_konwojsettingentries_5)))
  (bind _output_unitclass_3 (break `/Game/StrategyTrainer/Blueprints/Types/S_KonwojSettingEntry` (`|GetArrayItem` _settings_konwojsettingentries_2)))
  (bind (_output_blueunit_3 _output_redunit_3 _output_redunitactor) (break `/Game/StrategyTrainer/Blueprints/Types/S_BattleQueueEntry` (`|GetArrayItem` (`self.BattleQueue`))))
  (bind (_output_blueunit_4 _output_redunit_4) (break `/Game/StrategyTrainer/Blueprints/Types/S_BattleQueueEntry` (`|GetArrayItem` (`self.BattleQueue`))))
  (bind (_blueunitkillchance _redunitkillchance) (`/Game/StrategyTrainer/Blueprints/System/BFL_StrategyTrainer.GetUnitKillChance` _output_blueunit _output_redunit))
  (if (and (`KismetArrayLibrary.Array_IsValidIndex` _settings_konwojsettingentries) (`KismetArrayLibrary.Array_IsValidIndex` _battlequeue))
    (`|ExecutionSequence`
      (:`then_0`
        (if (<= (`KismetMathLibrary.RandomFloat`) _blueunitkillchance)
          (`KismetSystemLibrary.PrintString` "Blue unit -1 HP" false)
          (`self.SendToLogStatistics` (`KismetTextLibrary.Conv_StringToText` (`KismetStringLibrary.Concat_StrStr` "Defender hit" (`KismetSystemLibrary.GetClassDisplayName` _output_unitclass_2))))
          (`KismetArrayLibrary.Array_Set` _settings_konwojsettingentries_6 0 (make `/Game/StrategyTrainer/Blueprints/Types/S_KonwojSettingEntry` _output_unitclass (- _output_hp 1)))
          (`self.Hit`)
          (if (== _output_hp 0)
            (`self.SendToLogStatistics` (`KismetTextLibrary.Conv_StringToText` (`KismetStringLibrary.Concat_StrStr` "Defender killed" (`KismetSystemLibrary.GetClassDisplayName` _output_unitclass_3))))
            (`KismetArrayLibrary.Array_Remove` _settings_konwojsettingentries_3)
            (`self.OnDeath`)
            (`KismetSystemLibrary.PrintString` "Blue unit killed" false)
            (if (not (`KismetMathLibrary.Conv_IntToBool` (`KismetArrayLibrary.Array_Length` _settings_konwojsettingentries_3)))
              (`KismetSystemLibrary.DelayUntilNextTick`)
              (bind _returnvalue (`GameplayStatics.GetActorOfClass` "/Game/StrategyTrainer/Blueprints/Actors/BP_RoadSpline.BP_RoadSpline_C"))
              (`/Game/StrategyTrainer/Blueprints/Actors/BP_RoadSpline.ResetKonwoj` _returnvalue false)))))
      (:`then_1`
        (if (`KismetArrayLibrary.Array_IsValidIndex` (`self.BattleQueue`))
          (if (<= (`KismetMathLibrary.RandomFloat`) _redunitkillchance)
            (`self.SendToLogStatistics` (`KismetTextLibrary.Conv_StringToText` (`KismetStringLibrary.Concat_StrStr` "Convoy hit: " (`KismetSystemLibrary.GetClassDisplayName` _output_redunit_2))))
            (`KismetSystemLibrary.PrintString` "Red unit -1 HP" false)
            (`/Engine/EditorBlueprintResources/StandardMacros.IsValid` _output_redunitactor
              (:`Is Valid`
                (`/Game/StrategyTrainer/Blueprints/Actors/RedUnits/BP_RedUnit.Hit` _output_redunitactor)
                (bind _result (`/Engine/EditorBlueprintResources/StandardMacros.DecrementInt` (`/Game/StrategyTrainer/Blueprints/Actors/RedUnits/BP_RedUnit.HP` _output_redunitactor))
                  (:`  `
                    (if (== _result 0)
                      (`KismetSystemLibrary.PrintString` "Red unit killed" false)
                      (`self.SendToLogStatistics` (`KismetTextLibrary.Conv_StringToText` (`KismetStringLibrary.Concat_StrStr` "Convoy killed" (`KismetSystemLibrary.GetClassDisplayName` _output_redunit_4))))
                      (`/Game/StrategyTrainer/Blueprints/Actors/RedUnits/BP_RedUnit.OnDeath` _output_redunitactor)
                      (`self.SetLifeSpan` _output_redunitactor 0.2)))))))))
      (:`then_2`
        (if (`KismetArrayLibrary.Array_IsValidIndex` _battlequeue_2)
          (`KismetArrayLibrary.Array_Remove` _battlequeue_2))))))

(event `GetInfoAboutRedUnits`
  (bind _outactors (`GameplayStatics.GetAllActorsOfClass` "/Game/StrategyTrainer/Blueprints/Actors/RedUnits/BP_RedUnit.BP_RedUnit_C"))
  (bind _returnvalue (`STGameInstance.SortByDistance` _outactors))
  (set `self.RedUnits` _returnvalue))

(event `SendToLogStatistics`
  (params (InText :type Text))
  (bind _asgm_strategy_trainer (cast `/Game/StrategyTrainer/Blueprints/GameModes/GM_StrategyTrainer` (`GameplayStatics.GetGameMode`)))
  (bind _aswbp_statistics (cast `/Game/StrategyTrainer/Blueprints/UI/WBP_Statistics` (`WidgetComponent.GetWidget` (`/Game/StrategyTrainer/Blueprints/Actors/BP_Statistics.Widget` (`/Game/StrategyTrainer/Blueprints/GameModes/GM_StrategyTrainer.LogStatistics` _asgm_strategy_trainer)))))
  (`/Game/StrategyTrainer/Blueprints/UI/WBP_Statistics.AddEntry` _aswbp_statistics InText))

(fn `GetBonusPoints`
  (returns (Bonus :type "Float (double-precision)"))
  (bind _settings_konwojsettingentries (break `/Game/StrategyTrainer/Blueprints/Types/S_KonwojSettings` (`self.Settings`)))
  (bind _outactors (`GameplayStatics.GetAllActorsOfClass` "/Game/StrategyTrainer/Blueprints/Actors/RedUnits/BP_RedUnit.BP_RedUnit_C"))
  (return (+ (/ 200.0 (/ (`KismetArrayLibrary.Array_Length` _outactors) (`KismetArrayLibrary.Array_Length` (`/Game/StrategyTrainer/Blueprints/GameModes/GM_StrategyTrainer.StartRoundRedUnits` (cast `/Game/StrategyTrainer/Blueprints/GameModes/GM_StrategyTrainer` (`GameplayStatics.GetGameMode`) :!pure true))))) (* (`KismetArrayLibrary.Array_Length` _settings_konwojsettingentries) 50))))

(fn `MakeSettingsFromEnumArrayAndRun`
  (params (Enums :type "Array of /Game/StrategyTrainer/Blueprints/Types/E_BlueUnit Enum"))
  (locals (NewSettings :type "Array of /Game/StrategyTrainer/Blueprints/Types/S_KonwojSettingEntry Structure") (Log :type Text :default "NSLOCTEXT(\"[EF520965ACA618851ABD6250FDCF8567]\", \"240CA72D470A2A2873D4828AD6960886\", \"Chosen convoy: \")"))
  (for _array_element Enums
    (switch `/Game/StrategyTrainer/Blueprints/Types/E_BlueUnit` _array_element
      (:`NewEnumerator0`
        (`KismetArrayLibrary.Array_Add` (`local.NewSettings`) (make `/Game/StrategyTrainer/Blueprints/Types/S_KonwojSettingEntry` "/Game/StrategyTrainer/Blueprints/Actors/BlueUnits/BP_Tank.BP_Tank_C" 2)))
      (:`NewEnumerator1`
        (`KismetArrayLibrary.Array_Add` (`local.NewSettings`) (make `/Game/StrategyTrainer/Blueprints/Types/S_KonwojSettingEntry` "/Game/StrategyTrainer/Blueprints/Actors/BlueUnits/BP_BTR.BP_BTR_C" 2 "NewEnumerator1")))
      (:`NewEnumerator2`
        (`KismetArrayLibrary.Array_Add` (`local.NewSettings`) (make `/Game/StrategyTrainer/Blueprints/Types/S_KonwojSettingEntry` "/Game/StrategyTrainer/Blueprints/Actors/BlueUnits/BP_Piechota.BP_Piechota_C" 2 "NewEnumerator2")))
      (:`NewEnumerator3`
        (`KismetArrayLibrary.Array_Add` (`local.NewSettings`) (make `/Game/StrategyTrainer/Blueprints/Types/S_KonwojSettingEntry` "/Game/StrategyTrainer/Blueprints/Actors/BlueUnits/BP_Ciezarowka.BP_Ciezarowka_C" 2 "NewEnumerator3")))))
  (set `self.Settings` (make `/Game/StrategyTrainer/Blueprints/Types/S_KonwojSettings` (`local.NewSettings`)))
  (bind _asgm_strategy_trainer (cast `/Game/StrategyTrainer/Blueprints/GameModes/GM_StrategyTrainer` (`GameplayStatics.GetGameMode`)))
  (bind _aswbp_statistics (cast `/Game/StrategyTrainer/Blueprints/UI/WBP_Statistics` (`WidgetComponent.GetWidget` (`/Game/StrategyTrainer/Blueprints/Actors/BP_Statistics.Widget` (`/Game/StrategyTrainer/Blueprints/GameModes/GM_StrategyTrainer.Statistics` _asgm_strategy_trainer)))))
  (for _array_element_2 (`local.NewSettings`)
    (set `local.Log` (`KismetTextLibrary.Conv_StringToText` (`KismetStringLibrary.Concat_StrStr` (`KismetTextLibrary.Conv_TextToString` (`local.Log`)) (`KismetSystemLibrary.GetClassDisplayName` (break `/Game/StrategyTrainer/Blueprints/Types/S_KonwojSettingEntry` _array_element_2))))))
  (`/Game/StrategyTrainer/Blueprints/UI/WBP_Statistics.AddEntry` _aswbp_statistics (`local.Log`)))

(fn `UserConstructionScript`)