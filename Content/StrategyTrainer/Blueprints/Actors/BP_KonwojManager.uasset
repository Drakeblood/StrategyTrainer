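; Learning Agents manager actor that sets up PPO reinforcement learning for the convoy actor (BP_Konwoj), which it makes tick after itself.
; BeginPlay builds the interactor, policy and critic from Konwoj network assets, then a training environment and PPO trainer over a socket training process.
; RunTrainer runs training; RunInference only controls critic reinitialization, as its branch is empty.
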(event `self.ReceiveBeginPlay`
  (`|ExecutionSequence`
    (:`then_0`
      (bind _returnvalue (`GameplayStatics.GetActorOfClass` "/Game/StrategyTrainer/Blueprints/Actors/BP_Konwoj.BP_Konwoj_C"))
      (bind _output_get (set `self.Konwoj` _returnvalue))
      (`self.AddTickPrerequisiteActor` _output_get self))
    (:`then_2`
      (bind _returnvalue_2 (`LearningAgentsInteractor.MakeInteractor` (`self.LearningAgentsManager`) "/Game/StrategyTrainer/Blueprints/Agent/BP_KonwojLearningInteractor.BP_KonwojLearningInteractor_C" "KonwojInteractor"))
      (set `self.Interactor` _returnvalue_2))
    (:`then_3`
      (bind _returnvalue_3 (`LearningAgentsPolicy.MakePolicy` (`self.LearningAgentsManager`) (`self.Interactor`) "/Script/LearningAgents.LearningAgentsPolicy" "KonwojPolicy" "/Game/StrategyTrainer/Blueprints/Agent/DA_KonwojEncoder.DA_KonwojEncoder" "/Game/StrategyTrainer/Blueprints/Agent/DA_KonwojPolicy.DA_KonwojPolicy" "/Game/StrategyTrainer/Blueprints/Agent/DA_KonwojDecoder.DA_KonwojDecoder" false false false (`self.Policy Settings`)))
      (set `self.Policy` _returnvalue_3))
    (:`then_4`
      (bind _returnvalue_4 (`LearningAgentsCritic.MakeCritic` (`self.LearningAgentsManager`) (`self.Interactor`) (`self.Policy`) "/Script/LearningAgents.LearningAgentsCritic" "SportsCarCritic" "/Game/StrategyTrainer/Blueprints/Agent/DA_KonwojCritic.DA_KonwojCritic" (not (`self.RunInference`)) (`self.Critic Settings`)))
      (set `self.Critic` _returnvalue_4))
    (:`then_5`
      (bind _returnvalue_5 (`LearningAgentsTrainingEnvironment.MakeTrainingEnvironment` (`self.LearningAgentsManager`) "/Game/StrategyTrainer/Blueprints/Agent/BP_KonwojTraining.BP_KonwojTraining_C"))
      (set `self.TrainingEnvironment` _returnvalue_5)
      (bind _returnvalue_6 (`LearningAgentsCommunicatorLibrary.MakeSocketTrainingProcess` (`self.Trainer Process Settings`) (`self.Socket Settings`)))
      (bind _returnvalue_7 (`LearningAgentsPPOTrainer.MakePPOTrainer` (`self.LearningAgentsManager`) (`self.Interactor`) (`self.TrainingEnvironment`) (`self.Policy`) (`self.Critic`) _returnvalue_6 "/Game/StrategyTrainer/Blueprints/Agent/BP_KonwojTrainer.BP_KonwojTrainer_C" "PPOTrainer" (`self.Trainer Settings`)))
      (set `self.Trainer` _returnvalue_7))
    (:`then_6`
      (if (`self.RunInference`)
        _))))

(event `RunTrainer`
  (`LearningAgentsPPOTrainer.RunTraining` (`self.Trainer`) (struct :`NumberOfIterations` 1000000 :`LearningRatePolicy` 0.0001 :`LearningRateCritic` 0.001 :`LearningRateDecay` 1.0 :`WeightDecay` 0.0001 :`PolicyBatchSize` 1024 :`CriticBatchSize` 4096 :`PolicyWindowSize` 16 :`IterationsPerGather` 32 :`CriticWarmupIterations` 8 :`EpsilonClip` 0.2 :`ReturnRegularizationWeight` 0.0001 :`ActionSurrogateWeight` 1.0 :`ActionRegularizationWeight` 0.001 :`GaeLambda` 0.95 :`bAdvantageNormalization` true :`MaximumAdvantage` 10.0 :`GradNormMax` 0.5 :`RandomSeed` 1234 :`DiscountFactor` 0.99 :`Device` "GPU") (struct :`bUseFixedTimeStep` true :`FixedTimeStepFrequency` 60.0 :`bSetMaxPhysicsStepToFixedTimeStep` true :`bDisableMaxFPS` true :`bDisableVSync` true :`bDisableUseLessCPUInTheBackground` true :`bDisableEditorVSync` true) true true))

(fn `UserConstructionScript`)