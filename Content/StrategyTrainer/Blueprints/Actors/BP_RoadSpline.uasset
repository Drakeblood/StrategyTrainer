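; BP_RoadSpline is an actor that moves a referenced SplineActor along its spline from BeginPlay until it passes the last point.
; UpdateSpline advances distance by SplineSpeed and delta time, then re-calls itself through Delay Until Next Tick, clearing Move at the end.
; It applies the spline's local-space transform as the actor's location and rotation, with a -90 degree yaw offset.
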(event `self.ReceiveBeginPlay`
  (`self.UpdateSpline`))

(event `UpdateSpline`
  (set `self.Move` true)
  (bind _output_get (set `self.DistanceAlongSpline` (+ (* (`GameplayStatics.GetWorldDeltaSeconds`) (`self.SplineSpeed`)) (`self.DistanceAlongSpline`))))
  (if (> _output_get (`SplineComponent.GetDistanceAlongSplineAtSplinePoint` (`self.Spline`) (- (`SplineComponent.GetNumberOfSplinePoints` (`self.Spline`)) 1)))
    (set `self.Move` false)
    (else
      (bind _returnvalue (`SplineComponent.GetTransformAtDistanceAlongSpline` (`self.Spline`) _output_get "Local" false))
      (`self.K2_SetActorLocationAndRotation` (`self.SplineActor`) (`KismetMathLibrary.MakeVector` (.x (.location _returnvalue)) (.y (.location _returnvalue)) (.z (.location _returnvalue))) (`KismetMathLibrary.MakeRotator` (.roll (.rotation _returnvalue)) (.pitch (.rotation _returnvalue)) (+ (.yaw (.rotation _returnvalue)) -90.0)) false false)
      (`KismetSystemLibrary.DelayUntilNextTick`)
      (`self.UpdateSpline`))))

(fn `UserConstructionScript`)