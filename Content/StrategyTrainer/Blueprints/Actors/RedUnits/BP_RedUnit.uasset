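; Red (enemy) unit actor for the strategy trainer that queues battles against the convoy (BP_Konwoj) when it enters the attack sphere.
; Overlap passes a DoOnce, reset at each round end via the game mode, then adds BattleCount queue entries pairing the convoy's first configured unit class with this unit.
; Hit and death events spawn short-lived BP_AnimationMesh effects, with death playing a boom animation.
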(event `self.ReceiveBeginPlay`
  (add `/Game/StrategyTrainer/Blueprints/GameModes/GM_StrategyTrainer.OnRoundEnd` (cast `/Game/StrategyTrainer/Blueprints/GameModes/GM_StrategyTrainer` (`GameplayStatics.GetGameMode`) :!pure true) (delegate `OnRoundEnd_Event`))
  (bind _returnvalue (`GameplayStatics.GetActorOfClass` "/Game/StrategyTrainer/Blueprints/Actors/BP_Konwoj.BP_Konwoj_C"))
  (set `self.Konwoj` _returnvalue))

(event `OnRoundEnd_Event`
  (bind _settings_konwojsettingentries (break `/Game/StrategyTrainer/Blueprints/Types/S_KonwojSettings` (`/Game/StrategyTrainer/Blueprints/Actors/BP_Konwoj.Settings` (`self.Konwoj`))))
  (bind _output_unitclass (break `/Game/StrategyTrainer/Blueprints/Types/S_KonwojSettingEntry` (`|GetArrayItem` _settings_konwojsettingentries)))
  (goto _label :!via `Reset`))

(event `self.AttackSphere.OnComponentBeginOverlap`
  (params (OverlappedComponent :type "PrimitiveComponent Object Reference") (OtherActor :type "Actor Object Reference") (OtherComp :type "PrimitiveComponent Object Reference") (OtherBodyIndex :type Integer) (bFromSweep :type Boolean) (SweepResult :type "HitResult Structure (by ref)"))
  (bind _settings_konwojsettingentries (break `/Game/StrategyTrainer/Blueprints/Types/S_KonwojSettings` (`/Game/StrategyTrainer/Blueprints/Actors/BP_Konwoj.Settings` (`self.Konwoj`))))
  (bind _output_unitclass (break `/Game/StrategyTrainer/Blueprints/Types/S_KonwojSettingEntry` (`|GetArrayItem` _settings_konwojsettingentries)))
  (bind _asbp_konwoj (cast `/Game/StrategyTrainer/Blueprints/Actors/BP_Konwoj` OtherActor))
  (`/Engine/EditorBlueprintResources/StandardMacros.DoOnce` false :!label _label
    (:`Completed`
      (for _ (range 1 (+ (`self.BattleCount`) 1))
        (if (`KismetArrayLibrary.Array_IsValidIndex` _settings_konwojsettingentries)
          (`/Game/StrategyTrainer/Blueprints/Actors/BP_Konwoj.AddBattleQueue` _asbp_konwoj (make `/Game/StrategyTrainer/Blueprints/Types/S_BattleQueueEntry` _output_unitclass (`GameplayStatics.GetObjectClass` self) self)))))))

(event `OnDeath`
  (bind (_returnvalue_location _returnvalue_rotation) (`KismetMathLibrary.BreakTransform` (`SceneComponent.K2_GetComponentToWorld` (`self.Scene`))))
  (bind _returnvalue (`|SpawnActorFromClass` "/Game/StrategyTrainer/Blueprints/Actors/BP_AnimationMesh.BP_AnimationMesh_C" (`KismetMathLibrary.MakeTransform` _returnvalue_location _returnvalue_rotation) "AlwaysSpawn" "MultiplyWithRoot" null null))
  (`SkeletalMeshComponent.SetAnimation` (`/Game/StrategyTrainer/Blueprints/Actors/BP_AnimationMesh.SkeletalMesh` _returnvalue) "/Game/StrategyTrainer/Animations/Convoy_BoomPow_effect4_Anim_Boom.Convoy_BoomPow_effect4_Anim_Boom")
  (`self.SetLifeSpan` _returnvalue 0.5))

(event `Hit`
  (bind (_returnvalue_location _returnvalue_rotation) (`KismetMathLibrary.BreakTransform` (`SceneComponent.K2_GetComponentToWorld` (`self.Scene`))))
  (bind _returnvalue (`|SpawnActorFromClass` "/Game/StrategyTrainer/Blueprints/Actors/BP_AnimationMesh.BP_AnimationMesh_C" (`KismetMathLibrary.MakeTransform` _returnvalue_location _returnvalue_rotation) "AlwaysSpawn" "MultiplyWithRoot" null null))
  (`self.SetLifeSpan` _returnvalue 0.4))

(fn `UserConstructionScript`
  (`parent.UserConstructionScript`))