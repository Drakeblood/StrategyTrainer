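; Learning Agents interactor for BP_Konwoj (convoy) agents, exposing blue and red unit types to machine learning.
; Observes blue types from convoy settings and red types from its RedUnits as enum arrays, specified at max 8 but gathered at max 3.
; Declares enum-based actions for both sides.
; PerformAgentAction is unfinished: it only prints BlueUnits element names, with decoding and MakeSettingsFromEnumArrayAndRun left in disconnected experiments.
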(fn `GatherAgentObservation`
  (params (InObservationObject :type "LearningAgentsObservationObject Object Reference") (AgentId :type Integer))
  (returns (OutObservationObjectElement :type "LearningAgentsObservationObjectElement Structure"))
  (locals (ObsActor :type "/Game/StrategyTrainer/Blueprints/Actors/BP_Konwoj Object Reference") (BlueUnits :type "Array of LearningAgentsObservationObjectElement Structure") (RedUnits :type "Array of LearningAgentsObservationObjectElement Structure"))
  (bind _settings_konwojsettingentries (break `/Game/StrategyTrainer/Blueprints/Types/S_KonwojSettings` (`/Game/StrategyTrainer/Blueprints/Actors/BP_Konwoj.Settings` (`local.ObsActor`))))
  (set `local.ObsActor` (`self.GetAgent` AgentId "/Game/StrategyTrainer/Blueprints/Actors/BP_Konwoj.BP_Konwoj_C"))
  (for _array_element _settings_konwojsettingentries
    (`KismetArrayLibrary.Array_Add` (`local.BlueUnits`) (`LearningAgentsObservations.MakeEnumObservation` (`local.InObservationObject`) "/Game/StrategyTrainer/Blueprints/Types/E_BlueUnit.E_BlueUnit" (`.UnityType_8_641E3E9B417C57842903AC9DA51E534B` (break `/Game/StrategyTrainer/Blueprints/Types/S_KonwojSettingEntry` _array_element)) "EnumObservation" false null)))
  (for _array_element_2 (`/Game/StrategyTrainer/Blueprints/Actors/BP_Konwoj.RedUnits` (`local.ObsActor`))
    (`KismetArrayLibrary.Array_Add` (`local.RedUnits`) (`LearningAgentsObservations.MakeEnumObservation` (`local.InObservationObject`) "/Game/StrategyTrainer/Blueprints/Types/E_RedUnit.E_RedUnit" (`/Game/StrategyTrainer/Blueprints/Actors/RedUnits/BP_RedUnit.Type` (cast `/Game/StrategyTrainer/Blueprints/Actors/RedUnits/BP_RedUnit` _array_element_2 :!pure true)) "EnumObservation" false null)))
  (return (`LearningAgentsObservations.MakeStructObservation` (`local.InObservationObject`) (`|MakeMap` "BlueUnits" (`LearningAgentsObservations.MakeArrayObservation` (`local.InObservationObject`) (`local.BlueUnits`) 3) "RedUnits" (`LearningAgentsObservations.MakeArrayObservation` (`local.InObservationObject`) (`local.RedUnits`) 3) :!type "Name"))))

(fn `PerformAgentAction`
  (params (InActionObject :type "LearningAgentsActionObject Object Reference") (InActionObjectElement :type "LearningAgentsActionObjectElement Structure (by ref)") (AgentId :type Integer))
  (locals (ActActor :type "/Game/StrategyTrainer/Blueprints/Actors/BP_Konwoj Object Reference") (BlueUnits :type "Array of /Game/StrategyTrainer/Blueprints/Types/E_BlueUnit Enum"))
  (set `local.ActActor` (`self.GetAgent` AgentId "/Game/StrategyTrainer/Blueprints/Actors/BP_Konwoj.BP_Konwoj_C"))
  (bind _outelements (`LearningAgentsActions.GetStructAction` (`local.InActionObject`) (`local.InActionObjectElement`)))
  (bind (_outelementnames _outelements_2) (`LearningAgentsActions.GetStructActionToArrays` (`local.InActionObject`) (`BlueprintMapLibrary.Map_Find` _outelements "BlueUnits")))
  (for _array_element _outelementnames
    (`KismetSystemLibrary.PrintString` null (`KismetStringLibrary.Conv_NameToString` _array_element))))

(fn `SpecifyAgentAction`
  (params (InActionSchema :type "LearningAgentsActionSchema Object Reference"))
  (returns (OutActionSchemaElement :type "LearningAgentsActionSchemaElement Structure"))
  (bind _inactionschema (`local.InActionSchema`))
  (return (`LearningAgentsActions.SpecifyStructAction` (`local.InActionSchema`) (`|MakeMap` "BlueUnits" (`LearningAgentsActions.SpecifyEnumActionFromArray` _inactionschema "/Game/StrategyTrainer/Blueprints/Types/E_BlueUnit.E_BlueUnit") "RedUnits" (`LearningAgentsActions.SpecifyEnumAction` _inactionschema "/Game/StrategyTrainer/Blueprints/Types/E_RedUnit.E_RedUnit") :!type "Name"))))

(fn `SpecifyAgentObservation`
  (params (InObservationSchema :type "LearningAgentsObservationSchema Object Reference"))
  (returns (OutObservationSchemaElement :type "LearningAgentsObservationSchemaElement Structure"))
  (return (`LearningAgentsObservations.SpecifyStructObservation` (`local.InObservationSchema`) (`|MakeMap` "BlueUnits" (`LearningAgentsObservations.SpecifyArrayObservation` (`local.InObservationSchema`) (`LearningAgentsObservations.SpecifyEnumObservation` (`local.InObservationSchema`) "/Game/StrategyTrainer/Blueprints/Types/E_BlueUnit.E_BlueUnit") 8) "RedUnits" (`LearningAgentsObservations.SpecifyArrayObservation` (`local.InObservationSchema`) (`LearningAgentsObservations.SpecifyEnumObservation` (`local.InObservationSchema`) "/Game/StrategyTrainer/Blueprints/Types/E_RedUnit.E_RedUnit") 8) :!type "Name"))))