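; Learning Agents training environment for BP_Konwoj, the convoy agent that learns to travel along a road spline.
; Reward maps each agent's normalized distance along its RoadSpline to a -1 to 1 range and prints it; a velocity-along-spline reward node sits unused.
; Episode reset delegates to the RoadSpline's ResetKonwoj, and the completion check always returns Termination.
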(fn `GatherAgentCompletion`
  (params (AgentId :type Integer))
  (returns (OutCompletion :type "ELearningAgentsCompletion Enum"))
  (return "Termination"))

(fn `GatherAgentReward`
  (params (AgentId :type Integer))
  (returns (OutReward :type "Float (single-precision)"))
  (locals (RewardActor :type "/Game/StrategyTrainer/Blueprints/Actors/BP_Konwoj Object Reference"))
  (bind _spline (`/Game/StrategyTrainer/Blueprints/Actors/BP_RoadSpline.Spline` (`/Game/StrategyTrainer/Blueprints/Actors/BP_Konwoj.RoadSpline` (`local.RewardActor`))))
  (bind _returnvalue (`KismetMathLibrary.MapRangeClamped` (/ (`SplineComponent.GetDistanceAlongSplineAtLocation` _spline (`Actor.K2_GetActorLocation` (`local.RewardActor`)) "World") (`SplineComponent.GetSplineLength` _spline)) 0.0 1.0 -1.0 1.0))
  (set `local.RewardActor` (`self.GetAgent` AgentId "/Game/StrategyTrainer/Blueprints/Actors/BP_Konwoj.BP_Konwoj_C"))
  (`KismetSystemLibrary.PrintString` null (`KismetStringLibrary.Conv_DoubleToString` _returnvalue))
  (return _returnvalue))

(fn `ResetAgentEpisode`
  (params (AgentId :type Integer))
  (locals (Konwoj :type "/Game/StrategyTrainer/Blueprints/Actors/BP_Konwoj Object Reference"))
  (bind _output_get (set `local.Konwoj` (`self.GetAgent` AgentId "/Game/StrategyTrainer/Blueprints/Actors/BP_Konwoj.BP_Konwoj_C")))
  (`/Game/StrategyTrainer/Blueprints/Actors/BP_RoadSpline.ResetKonwoj` (`/Game/StrategyTrainer/Blueprints/Actors/BP_Konwoj.RoadSpline` _output_get) true))