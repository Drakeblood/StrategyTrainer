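; Game mode for the StrategyTrainer game that links the road spline and the convoy used in a simulation.
; On BeginPlay it finds and caches the level's BP_RoadSpline and BP_Konwoj actors.
; RunSimulation starts the run from the beginning of the road.
; A disconnected node chain that would fill the convoy settings with tanks and infantry never executes.
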(event `self.ReceiveBeginPlay`
  (bind _returnvalue (`GameplayStatics.GetActorOfClass` "/Game/StrategyTrainer/Blueprints/Actors/BP_RoadSpline.BP_RoadSpline_C"))
  (set `self.Road` _returnvalue)
  (bind _returnvalue_2 (`GameplayStatics.GetActorOfClass` "/Game/StrategyTrainer/Blueprints/Actors/BP_Konwoj.BP_Konwoj_C"))
  (set `self.Konwoj` _returnvalue_2))

(event `RunSimulation`
  (`/Game/StrategyTrainer/Blueprints/Actors/BP_RoadSpline.RunFromStart` (`self.Road`)))

(fn `UserConstructionScript`)