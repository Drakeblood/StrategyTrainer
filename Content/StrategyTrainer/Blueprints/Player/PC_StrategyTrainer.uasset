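; Player controller for the strategy trainer, spawning the HUD and a cursor actor that follows the mouse trace while the unit context menu is hidden.
; Left click toggles that menu and the mouse pointer; S cycles global time dilation to speed up play.
; Space runs the BP_KonwojManager trainer once per round, re-armed by the game mode's round-end event.
; L starts continuous training by also binding a rerun to each round end.
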(event `Key|SpaceBar`
  (params (Key :type "Key Structure"))
  (:`Pressed`
    (`/Engine/EditorBlueprintResources/StandardMacros.DoOnce` false :!label _label
      (:`Completed`
        (bind _returnvalue (`GameplayStatics.GetActorOfClass` "/Game/StrategyTrainer/Blueprints/Actors/BP_KonwojManager.BP_KonwojManager_C"))
        (`/Game/StrategyTrainer/Blueprints/Actors/BP_KonwojManager.RunTrainer` _returnvalue)))))

(event `OnRoundEnd_Event`
  (goto _label :!via `Reset`))

(event `self.ReceiveBeginPlay`
  (bind _returnvalue (`|SpawnActorFromClass` "/Game/StrategyTrainer/Blueprints/Player/BP_Cursor.BP_Cursor_C" (`KismetMathLibrary.MakeTransform` (`.Location` (`GameplayStatics.BreakHitResult` (`self.GetHitResultUnderCursorByChannel` "TraceTypeQuery1")))) "AlwaysSpawn" "MultiplyWithRoot" null null))
  (set `self.Cursor` _returnvalue)
  (bind _returnvalue_2 (`|CreateWidget` "/Game/StrategyTrainer/Blueprints/UI/WBP_HUD.WBP_HUD_C"))
  (bind _output_get (set `self.HUD` _returnvalue_2))
  (`UserWidget.AddToViewport` _output_get 0)
  (add `/Game/StrategyTrainer/Blueprints/GameModes/GM_StrategyTrainer.OnRoundEnd` (cast `/Game/StrategyTrainer/Blueprints/GameModes/GM_StrategyTrainer` (`GameplayStatics.GetGameMode`) :!pure true) (delegate `OnRoundEnd_Event`)))

(event `self.ReceiveTick`
  (params (DeltaSeconds :type "Float (single-precision)"))
  (if (`|EnumEquality` (`Widget.Visibility` (`/Game/StrategyTrainer/Blueprints/UI/WBP_HUD.WBP_UnitContextMenu` (`self.HUD`))) "Hidden")
    (`self.K2_SetActorLocation` (`self.Cursor`) (`.Location` (`GameplayStatics.BreakHitResult` (`self.GetHitResultUnderCursorByChannel` "TraceTypeQuery1"))) false false)))

(event `Key|LeftMouseButton`
  (params (Key :type "Key Structure"))
  (bind _wbp_unitcontextmenu (`/Game/StrategyTrainer/Blueprints/UI/WBP_HUD.WBP_UnitContextMenu` (`self.HUD`)))
  (:`Pressed`
    (if (`|EnumEquality` (`Widget.Visibility` _wbp_unitcontextmenu) "Hidden")
      (set `self.bShowMouseCursor` true)
      (`Widget.SetVisibility` _wbp_unitcontextmenu "Visible")
      (else
        (set `self.bShowMouseCursor` false)
        (`Widget.SetVisibility` _wbp_unitcontextmenu "Hidden")))))

(event `Key|S`
  (params (Key :type "Key Structure"))
  (:`Pressed`
    (if (> (`GameplayStatics.GetGlobalTimeDilation`) 2.0)
      (`GameplayStatics.SetGlobalTimeDilation` 1.0)
      (elif (> (`GameplayStatics.GetGlobalTimeDilation`) 1.0)
        (`GameplayStatics.SetGlobalTimeDilation` 4.0)
        (else
          (`GameplayStatics.SetGlobalTimeDilation` 2.0))))))

(event `Key|L`
  (params (Key :type "Key Structure"))
  (:`Pressed`
    (bind _returnvalue (`GameplayStatics.GetActorOfClass` "/Game/StrategyTrainer/Blueprints/Actors/BP_KonwojManager.BP_KonwojManager_C"))
    (`/Game/StrategyTrainer/Blueprints/Actors/BP_KonwojManager.RunTrainer` _returnvalue)
    (add `/Game/StrategyTrainer/Blueprints/GameModes/GM_StrategyTrainer.OnRoundEnd` (cast `/Game/StrategyTrainer/Blueprints/GameModes/GM_StrategyTrainer` (`GameplayStatics.GetGameMode`) :!pure true) (delegate `OnRoundEnd`))))

(event `OnRoundEnd`
  (bind _returnvalue (`GameplayStatics.GetActorOfClass` "/Game/StrategyTrainer/Blueprints/Actors/BP_KonwojManager.BP_KonwojManager_C"))
  (`/Game/StrategyTrainer/Blueprints/Actors/BP_KonwojManager.RunTrainer` _returnvalue))

(fn `UserConstructionScript`)