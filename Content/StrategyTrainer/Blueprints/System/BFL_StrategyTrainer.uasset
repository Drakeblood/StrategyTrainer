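; Blueprint function library for the strategy trainer that supplies combat odds for a matchup between a Blue unit and a Red unit.
; GetUnitKillChance returns a Blue and a Red kill chance for each pairing of tank, infantry, BTR or truck against anti-tank, mines, machine-gun nest or sniper.
; The table is hardcoded as a nested branch chain on unit type, and unlisted pairings return the local variables' defaults.
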(fn `GetUnitKillChance`
  (params (BlueUnit :type "/Game/StrategyTrainer/Blueprints/Actors/BlueUnits/BP_BlueUnit Class Reference") (RedUnit :type "/Game/StrategyTrainer/Blueprints/Actors/RedUnits/BP_RedUnit Class Reference"))
  (returns (BlueUnitKillChance :type "Float (double-precision)") (RedUnitKillChance :type "Float (double-precision)"))
  (locals (LBlueUnitKillChance :type "Float (double-precision)" :default 0.0) (LRedUnitKillChance :type "Float (double-precision)" :default 0.0))
  (`|ExecutionSequence`
    (:`then_0`
      ; Tank
      (if (and (== (`local.BlueUnit`) "/Game/StrategyTrainer/Blueprints/Actors/BlueUnits/BP_Tank.BP_Tank_C") (== (`local.RedUnit`) "/Game/StrategyTrainer/Blueprints/Actors/RedUnits/BP_AntiTank.BP_AntiTank_C"))
        (set `local.LRedUnitKillChance` 0.2)
        (set `local.LBlueUnitKillChance` 0.8)
        (elif (and (== (`local.BlueUnit`) "/Game/StrategyTrainer/Blueprints/Actors/BlueUnits/BP_Tank.BP_Tank_C") (== (`local.RedUnit`) "/Game/StrategyTrainer/Blueprints/Actors/RedUnits/BP_MediumMines.BP_MediumMines_C"))
          (set `local.LRedUnitKillChance` 0.5)
          (set `local.LBlueUnitKillChance` 0.5)
          (elif (and (== (`local.BlueUnit`) "/Game/StrategyTrainer/Blueprints/Actors/BlueUnits/BP_Tank.BP_Tank_C") (== (`local.RedUnit`) "/Game/StrategyTrainer/Blueprints/Actors/RedUnits/BP_GniazdoMaszynowe.BP_GniazdoMaszynowe_C"))
            (set `local.LRedUnitKillChance` 0.9)
            (set `local.LBlueUnitKillChance` 0.1)
            (elif (and (== (`local.BlueUnit`) "/Game/StrategyTrainer/Blueprints/Actors/BlueUnits/BP_Tank.BP_Tank_C") (== (`local.RedUnit`) "/Game/StrategyTrainer/Blueprints/Actors/RedUnits/BP_Sniper.BP_Sniper_C"))
              (set `local.LRedUnitKillChance` 0.1)
              (set `local.LBlueUnitKillChance` 0.0)
              (else
                ; Piechota
                (if (and (== (`local.BlueUnit`) "/Game/StrategyTrainer/Blueprints/Actors/BlueUnits/BP_Piechota.BP_Piechota_C") (== (`local.RedUnit`) "/Game/StrategyTrainer/Blueprints/Actors/RedUnits/BP_AntiTank.BP_AntiTank_C"))
                  (set `local.LRedUnitKillChance` 0.9)
                  (set `local.LBlueUnitKillChance` 0.1)
                  (elif (and (== (`local.BlueUnit`) "/Game/StrategyTrainer/Blueprints/Actors/BlueUnits/BP_Piechota.BP_Piechota_C") (== (`local.RedUnit`) "/Game/StrategyTrainer/Blueprints/Actors/RedUnits/BP_MediumMines.BP_MediumMines_C"))
                    (set `local.LRedUnitKillChance` 0.6)
                    (set `local.LBlueUnitKillChance` 0.4)
                    (elif (and (== (`local.BlueUnit`) "/Game/StrategyTrainer/Blueprints/Actors/BlueUnits/BP_Piechota.BP_Piechota_C") (== (`local.RedUnit`) "/Game/StrategyTrainer/Blueprints/Actors/RedUnits/BP_GniazdoMaszynowe.BP_GniazdoMaszynowe_C"))
                      (set `local.LRedUnitKillChance` 0.1)
                      (set `local.LBlueUnitKillChance` 0.9)
                      (elif (and (== (`local.BlueUnit`) "/Game/StrategyTrainer/Blueprints/Actors/BlueUnits/BP_Piechota.BP_Piechota_C") (== (`local.RedUnit`) "/Game/StrategyTrainer/Blueprints/Actors/RedUnits/BP_Sniper.BP_Sniper_C"))
                        (set `local.LRedUnitKillChance` 0.0)
                        (set `local.LBlueUnitKillChance` 0.5)
                        (else
                          ; BTR
                          (if (and (== (`local.BlueUnit`) "/Game/StrategyTrainer/Blueprints/Actors/BlueUnits/BP_BTR.BP_BTR_C") (== (`local.RedUnit`) "/Game/StrategyTrainer/Blueprints/Actors/RedUnits/BP_AntiTank.BP_AntiTank_C"))
                            (set `local.LRedUnitKillChance` 0.4)
                            (set `local.LBlueUnitKillChance` 0.6)
                            (elif (and (== (`local.BlueUnit`) "/Game/StrategyTrainer/Blueprints/Actors/BlueUnits/BP_BTR.BP_BTR_C") (== (`local.RedUnit`) "/Game/StrategyTrainer/Blueprints/Actors/RedUnits/BP_MediumMines.BP_MediumMines_C"))
                              (set `local.LRedUnitKillChance` 0.2)
                              (set `local.LBlueUnitKillChance` 0.8)
                              (elif (and (== (`local.BlueUnit`) "/Game/StrategyTrainer/Blueprints/Actors/BlueUnits/BP_BTR.BP_BTR_C") (== (`local.RedUnit`) "/Game/StrategyTrainer/Blueprints/Actors/RedUnits/BP_GniazdoMaszynowe.BP_GniazdoMaszynowe_C"))
                                (set `local.LRedUnitKillChance` 0.8)
                                (set `local.LBlueUnitKillChance` 0.2)
                                (elif (and (== (`local.BlueUnit`) "/Game/StrategyTrainer/Blueprints/Actors/BlueUnits/BP_BTR.BP_BTR_C") (== (`local.RedUnit`) "/Game/StrategyTrainer/Blueprints/Actors/RedUnits/BP_Sniper.BP_Sniper_C"))
                                  (set `local.LRedUnitKillChance` 0.8)
                                  (set `local.LBlueUnitKillChance` 0.0)
                                  (else
                                    ; Ciezarowka
                                    (if (and (== (`local.BlueUnit`) "/Game/StrategyTrainer/Blueprints/Actors/BlueUnits/BP_Ciezarowka.BP_Ciezarowka_C") (== (`local.RedUnit`) "/Game/StrategyTrainer/Blueprints/Actors/RedUnits/BP_AntiTank.BP_AntiTank_C"))
                                      (set `local.LRedUnitKillChance` 0.0)
                                      (set `local.LBlueUnitKillChance` 0.8)
                                      (elif (and (== (`local.BlueUnit`) "/Game/StrategyTrainer/Blueprints/Actors/BlueUnits/BP_Ciezarowka.BP_Ciezarowka_C") (== (`local.RedUnit`) "/Game/StrategyTrainer/Blueprints/Actors/RedUnits/BP_MediumMines.BP_MediumMines_C"))
                                        (set `local.LRedUnitKillChance` 0.0)
                                        (set `local.LBlueUnitKillChance` 0.5)
                                        (elif (and (== (`local.BlueUnit`) "/Game/StrategyTrainer/Blueprints/Actors/BlueUnits/BP_Ciezarowka.BP_Ciezarowka_C") (== (`local.RedUnit`) "/Game/StrategyTrainer/Blueprints/Actors/RedUnits/BP_GniazdoMaszynowe.BP_GniazdoMaszynowe_C"))
                                          (set `local.LRedUnitKillChance` 0.0)
                                          (set `local.LBlueUnitKillChance` 0.2)
                                          (elif (and (== (`local.BlueUnit`) "/Game/StrategyTrainer/Blueprints/Actors/BlueUnits/BP_Ciezarowka.BP_Ciezarowka_C") (== (`local.RedUnit`) "/Game/StrategyTrainer/Blueprints/Actors/RedUnits/BP_Sniper.BP_Sniper_C"))
                                            (set `local.LRedUnitKillChance` 0.0)
                                            (set `local.LBlueUnitKillChance` 0.1)))))))))))))))))))))
    (:`then_1`
      (return (`local.LBlueUnitKillChance`) (`local.LRedUnitKillChance`)))))